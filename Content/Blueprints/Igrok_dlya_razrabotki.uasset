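; Development player Blueprint with first-person-style movement, look and interaction controls.
; Axis inputs move it along the actor's forward and right vectors and drive controller yaw and inverted pitch.
; Pressing E runs a debug-drawn Visibility line trace a short distance along Camera1's forward vector and sends InteractMessage to the hit actor.
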(event Input|AxisEvents|InputAxisMoveForward
  (params (AxisValue :type Float%20%28single-precision%29))
  ;[1 1 1] Перемещение
  (Pawn|Input|AddMovementInput (Transformation|GetActorForwardVector) AxisValue false))

(event Input|AxisEvents|InputAxisMoveRight
  (params (AxisValue :type Float%20%28single-precision%29))
  ;[1 1 1] Перемещение
  (Pawn|Input|AddMovementInput (Transformation|GetActorRightVector) AxisValue false))

(event Input|AxisEvents|InputAxisLookHorizontal
  (params (AxisValue :type Float%20%28single-precision%29))
  ;[1 1 1] Обзор в пространстве
  (Pawn|Input|AddControllerYawInput AxisValue))

(event Input|AxisEvents|InputAxisLookVertical
  (params (AxisValue :type Float%20%28single-precision%29))
  ;[1 1 1] Обзор в пространстве
  (Pawn|Input|AddControllerPitchInput (* AxisValue -1.0)))

(event Input|KeyboardEvents|E
  (params (Key :type Key%20Structure :default "None"))
  (bind _camera1 (Variables|Default|GetCamera1))
  (bind _returnvalue (Transformation|GetWorldLocation _camera1))
  ;[1 1 1] Трасировка лучей
  (:Pressed
    (bind (_outhit _returnvalue_2) (Collision|LineTraceByChannel _returnvalue (+ _returnvalue (* (Math|Vector|GetForwardVector _camera1) 5e+02)) "TraceTypeQuery1" false 0 "ForDuration"))
    (if _returnvalue_2
      (Class|BPC|Interact(Message) (.HitActor (Collision|BreakHitResult _outhit))))))

(fn ConstructionScript)