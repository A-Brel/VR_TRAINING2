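; DOOR_RU04 is an interactable door that swings the RU04 component between two rotations.
; Interact plays or reverses a timeline according to the OpenDoorStatus flag.
; The timeline's Driver track blends relative rotation from StartDoor to EndDoor, and the flag toggles only when the timeline finishes.
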(event EventInteract
  (if (Variables|Default|GetOpenDoorStatus)
    (bind _driver (Timeline|Timeline_0 Play)
      (:Update
        (Transformation|SetRelativeRotation (Variables|Default|GetRU-0_4) (Math|Rotator|Lerp(Rotator) (Variables|Default|GetStartDoor) (Variables|Default|GetEndDoor) _driver) false false))
      (:Finished
        (if (Variables|Default|GetOpenDoorStatus)
          (Variables|Default|SetOpenDoorStatus false)
          (else
            (Variables|Default|SetOpenDoorStatus true)))))
    (else
      (Timeline|Timeline_0 Reverse))))

(fn ConstructionScript)